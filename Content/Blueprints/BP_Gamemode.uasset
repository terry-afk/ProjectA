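; Game mode Blueprint that manages enemy spawn pacing and the enemy population count.
; An interface event carrying an enemy spawner starts a looping timer at an interval derived from SpawnSpeed, though the timer's bound event is not defined here.
; Increment and decrement events maintain EnemyCount.
; CanSpawnEnemy compares that count to EnemyMax with less-or-equal, so it still returns true at the maximum.
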(event `self.ReceiveBeginPlay`)

(event `/Game/Blueprints/BPI_GameManager_Enemy.EnemySpawnerInterface`
  (params (EnemySpawner :type "/Game/Blueprints/BP_SpawnEnemy Object Reference"))
  ;[1 1 1] Spawn Enemy
  (`KismetSystemLibrary.K2_SetTimerDelegate` (`|CreateDelegate` EnemySpawner :!event `SpawnEnemy`) (/ 1.0 (`self.Spawn Speed`)) true))

(event `/Game/Blueprints/BPI_GameManager_Enemy.IncrementEnemyCount`
  (`/Engine/EditorBlueprintResources/StandardMacros.IncrementInt` (`self.EnemyCount`)))

(event `/Game/Blueprints/BPI_GameManager_Enemy.DecrementEnemyCount`
  (`/Engine/EditorBlueprintResources/StandardMacros.DecrementInt` (`self.EnemyCount`)))

(fn `CanSpawnEnemy`
  (returns (CanSpawn :type Boolean))
  (return (<= (`self.EnemyCount`) (`self.EnemyMax`))))

(fn `UserConstructionScript`)