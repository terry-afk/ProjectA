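; BP_FireBall_Manager is a levelled bonus actor that spawns and upgrades attached BP_FireBall actors, with root rotation kept absolute.
; GainLevel increments Level until the combined map maximum, though clamped to MapLevel's length, then calls SpawnNewBalls.
; A MapLevel entry adds a ball at that transform; otherwise MapLevelDamage sets damage on every BP_FireBall in the world.
; GetNextUpgrade reports whether the next level grants a ball or damage.
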(event `self.ReceiveBeginPlay`
  (`SceneComponent.SetAbsolute` (`self.DefaultSceneRoot`) false true false))

(event `Spawn new balls`
  (bind (_value _returnvalue) (`BlueprintMapLibrary.Map_Find` (`self.MapLevel`) (`self.Level`)))
  (bind (_value_2 _returnvalue_2) (`BlueprintMapLibrary.Map_Find` (`self.MapLevelDamage`) (`self.Level`)))
  (if _returnvalue
    (bind _returnvalue_3 (`|SpawnActorFromClass` "/Game/Blueprints/Bonus/BP_FireBall.BP_FireBall_C" (`KismetMathLibrary.Conv_VectorToTransform` _value) "Undefined" "MultiplyWithRoot" null (stale _output_get) null))
    (`self.K2_AttachToActor` _returnvalue_3 self "None" "KeepRelative" "KeepRelative" "KeepRelative" true)
    (elif _returnvalue_2
      (bind _output_get (set `self.Damage` _value_2))
      (bind _outactors (`GameplayStatics.GetAllActorsOfClass` "/Game/Blueprints/Bonus/BP_FireBall.BP_FireBall_C"))
      (for _array_element _outactors
        (set `/Game/Blueprints/Bonus/BP_FireBall.Damage` (`self.Damage`) _array_element))
      (else
        (`KismetSystemLibrary.PrintString` "ERROR WHILE GETTING A LEVEL")))))

(event `Gain Level`
  (bind _ismaxlevel (`self.Is Max Level`))
  (if (not _ismaxlevel)
    (bind _output_get (set `self.Level` (`KismetMathLibrary.Clamp` (+ (`self.Level`) 1) 0 (`BlueprintMapLibrary.Map_Length` (`self.MapLevel`)))))
    (`self.Spawn new balls`)
    (`KismetSystemLibrary.PrintString` (`KismetStringLibrary.Conv_IntToString` _output_get))))

(fn `Get Max Level`
  (returns (`Max Level` :type Integer))
  (return (+ (- (`BlueprintMapLibrary.Map_Length` (`self.MapLevel`)) 1) (- (`BlueprintMapLibrary.Map_Length` (`self.MapLevelDamage`)) 1))))

(fn `Get Next upgrade`
  (returns (Ball :type Boolean) (Damage :type "Float (double-precision)"))
  (if (`.ReturnValue` (`BlueprintMapLibrary.Map_Find` (`self.MapLevel`) (+ (`self.Level`) 1)))
    (return true 0.0)
    (else
      (return false (`BlueprintMapLibrary.Map_Find` (`self.MapLevelDamage`) (+ (`self.Level`) 1))))))

(fn `Is Max Level`
  (returns (IsMaxLevel :type Boolean))
  (bind _max_level (`self.Get Max Level`))
  (return (== _max_level (`self.Level`))))

(fn `UserConstructionScript`)