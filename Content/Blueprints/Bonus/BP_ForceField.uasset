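; Force field bonus that periodically shows a collidable sphere shield for a duration set by its level.
; A looping timer, its interval fixed at BeginPlay as ReloadTime minus the current duration, triggers activation, then a Delay hides the sphere and disables its collision.
; MapLevel maps each level to an uptime, which GainLevel raises by a clamped Level increment.
; Helper functions report whether the level is maxed and the next upgrade's value.
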(event `self.ReceiveBeginPlay`
  (`KismetSystemLibrary.PrintString` "JE SUIS LA")
  (`self.Handle Sphere` true)
  (`KismetSystemLibrary.K2_SetTimerDelegate` (delegate `Activate Shield`) (- (`self.ReloadTime`) (`BlueprintMapLibrary.Map_Find` (`self.MapLevel`) (`self.Level`))) true))

(event `Activate Shield`
  ;[1 1 1] Activate shield event
  (bind _output_get (set `self.TimeUp` (`BlueprintMapLibrary.Map_Find` (`self.MapLevel`) (`self.Level`))))
  (`self.Handle Sphere` false)
  (`KismetSystemLibrary.Delay` _output_get)
  (`self.Handle Sphere` true))

(event `Handle Sphere`
  (params (Hide :type Boolean))
  (bind _sphere (`self.Sphere`))
  ;[1 1 1] Handle sphere spawn
  (`SceneComponent.SetHiddenInGame` _sphere Hide false)
  (if Hide
    (`PrimitiveComponent.SetCollisionEnabled` _sphere "NoCollision")
    (else
      (`PrimitiveComponent.SetCollisionEnabled` (`self.Sphere`) "QueryAndPhysics"))))

(event `Gain Level`
  ;[1 1 1] Gain level
  (set `self.Level` (`KismetMathLibrary.Clamp` (+ (`self.Level`) 1) 0 (- (`BlueprintMapLibrary.Map_Length` (`self.MapLevel`)) 1))))

(fn `Get Next Upgrade`
  (returns (UpTime :type "Float (double-precision)"))
  (bind _maplevel (`self.MapLevel`))
  (return (`BlueprintMapLibrary.Map_Find` _maplevel (`KismetMathLibrary.Clamp` (+ (`self.Level`) 1) 0 (- (`BlueprintMapLibrary.Map_Length` _maplevel) 1)))))

(fn `Is Max Level`
  (returns (IsMaxLevel :type Boolean))
  (return (== (- (`BlueprintMapLibrary.Map_Length` (`self.MapLevel`)) 1) (`self.Level`))))

(fn `UserConstructionScript`)