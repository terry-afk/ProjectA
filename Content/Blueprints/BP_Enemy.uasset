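; Enemy Blueprint that chases the first player pawn and plays a spider attack montage on reaching it.
; A looping timer started at BeginPlay reissues AIMoveTo, and each successful move triggers the attack.
; CanAttack gates the attack but is restored as soon as the montage starts, not when it completes.
; HpUpdate adds a signed amount to Hp and sets a death flag at zero or below, exposed through GetIsDead.
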(event `self.ReceiveBeginPlay`
  (`KismetSystemLibrary.K2_SetTimerDelegate` (delegate `ChasePlayer`) 1.0 true))

(event `ChasePlayer`
  (`|AIMoveTo` self (0.0 0.0 0.0) (`GameplayStatics.GetPlayerPawn` 0)
    (:`OnSuccess`
      (`self.Attack`))))

(event `Attack`
  (if (`self.CanAttack`)
    (set `self.CanAttack` false)
    (`|PlayMontage` (`self.Mesh`) "/Game/Blueprints/AM_SpiderAttack.AM_SpiderAttack"
      (:`then`
        (set `self.CanAttack` true)))))

(fn `GetIsDead`
  (returns (IsDead :type Boolean))
  (return (`self.IsDead`)))

(fn `HpUpdate`
  (params (Domage :type Integer))
  (bind _output_get (set `self.Hp` (+ Domage (`self.Hp`))))
  (if (<= _output_get 0)
    (set `self.IsDead` true)
    (else
      (return))))

(fn `UserConstructionScript`)