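; BP_SpawnSpider is a spawn-volume actor that creates spider enemies inside its box.
; On BeginPlay it registers itself with the game mode through an interface message.
; Its SpawnSpider event asks the game mode whether spawning is allowed, then spawns a BP_Enemy AI at a random point within the box and tells the game mode to increment the spider count.
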(event `self.ReceiveBeginPlay`
  (message `/Game/Blueprints/BPI_GameManager_Spider.SpiderSpawnerInterface` (`GameplayStatics.GetGameMode`) self))

(event `SpawnSpider`
  (bind _box (`self.Box`))
  (bind _canspawn (message `/Game/Blueprints/BPI_GameManager_Spider.CanSpawnSpider` (`GameplayStatics.GetGameMode`)))
  (if _canspawn
    (`AIBlueprintHelperLibrary.SpawnAIFromClass` "/Game/Blueprints/BP_Enemy.BP_Enemy_C" null (`KismetMathLibrary.RandomPointInBoundingBox` (`SceneComponent.K2_GetComponentLocation` _box) (`BoxComponent.GetScaledBoxExtent` _box)) (struct) false null)
    (message `/Game/Blueprints/BPI_GameManager_Spider.IncrementSpiderCount` (`GameplayStatics.GetGameMode`))))

(fn `UserConstructionScript`)