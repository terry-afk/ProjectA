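; Enemy character Blueprint that chases the player, deals melee and contact damage, and drops XP on death.
; A looping timer reissues AI MoveTo toward the player, and reaching them triggers a gated attack montage that damages BP_Hero on completion.
; Capsule overlap with the hero also deals damage with a punch sound.
; TakeDamage feeds HpUpdate, whose death event spawns an XP orb, notifies the game mode and destroys the actor.
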(event `self.ReceiveBeginPlay`
  (`KismetSystemLibrary.K2_SetTimerDelegate` (delegate `ChasePlayer`) 1.0 true))

(event `ChasePlayer`
  (`|AIMoveTo` self (0.0 0.0 0.0) (`GameplayStatics.GetPlayerPawn` 0)
    (:`OnSuccess`
      (`self.Attack`))))

(event `Attack`
  (if (`self.CanAttack`)
    (set `self.CanAttack` false)
    (`|PlayMontage` (`self.Mesh`) (`self.AnimationAttack`)
      (:`OnCompleted`
        (set `self.CanAttack` true)
        (bind _asbp_hero (cast `/Game/Blueprints/BP_Hero` (`GameplayStatics.GetPlayerPawn` 0)))
        (`/Game/Blueprints/BP_Hero.TakeDamage` _asbp_hero 10.0)))))

(event `IsDead`
  (`|SpawnActorFromClass` "/Game/Blueprints/XPOrb.XPOrb_C" (`SceneComponent.K2_GetComponentToWorld` (`self.Mesh`)) "Undefined" "MultiplyWithRoot" null (`self.XpGain`) null)
  (message `/Game/Blueprints/BPI_GameManager_Enemy.DecrementEnemyCount` (`GameplayStatics.GetGameMode`))
  (`self.K2_DestroyActor`))

(event `self.CapsuleComponent.OnComponentBeginOverlap`
  (params (OverlappedComponent :type "PrimitiveComponent Object Reference") (OtherActor :type "Actor Object Reference") (OtherComp :type "PrimitiveComponent Object Reference") (OtherBodyIndex :type Integer) (bFromSweep :type Boolean) (SweepResult :type "HitResult Structure (by ref)"))
  (bind _asbp_hero (cast `/Game/Blueprints/BP_Hero` OtherActor))
  (`/Game/Blueprints/BP_Hero.TakeDamage` _asbp_hero (`self.Damage`))
  (`GameplayStatics.PlaySoundAtLocation` "/Game/Sound/punch-140236.punch-140236" (`SceneComponent.K2_GetComponentLocation` (`self.CapsuleComponent`)) (struct) 0.3 1.0 0.0 null null null null))

(fn `HpUpdate`
  (params (Domage :type "Float (double-precision)"))
  (bind _output_get (set `self.Hp` (+ Domage (`self.Hp`))))
  (if (<= _output_get 0)
    (`self.IsDead`)
    (else
      (return))))

(fn `Take Damage`
  (params (Damage :type "Float (double-precision)"))
  (bind _result (`/Engine/EditorBlueprintResources/StandardMacros.NegateFloat` (`KismetMathLibrary.Abs` Damage))
    (:`  `
      (`self.HpUpdate` _result))))

(fn `UserConstructionScript`)