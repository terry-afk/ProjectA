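; Enemy spawner actor that spawns endlessly recurring, escalating waves of goblins inside its box volume.
; On BeginPlay it messages the GameMode and starts a looping timer that calls SpawnWave.
; Each wave increments WaveLevel, scaling goblin count and HP linearly, while UpdateXpGain triples the XP reward every five levels.
; SpawnEnemy places each AI goblin at a random point, sets its stats and increments the GameMode's enemy count.
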(event `self.ReceiveBeginPlay`
  (message `/Game/Blueprints/BPI_GameManager_Enemy.EnemySpawnerInterface` (`GameplayStatics.GetGameMode`) self)
  (message `/Game/Blueprints/BPI_GameManager_Enemy.HandleSpawnWave` (`GameplayStatics.GetGameMode`) self)
  (`KismetSystemLibrary.K2_SetTimerDelegate` (delegate `Spawn Wave`) (`self.TimerSpawnWave`) true))

(event `SpawnEnemy`
  (bind _box (`self.Box`))
  (`KismetSystemLibrary.PrintString` "Je spawn un ennemi")
  (bind _returnvalue (`AIBlueprintHelperLibrary.SpawnAIFromClass` "/Game/Blueprints/Ennemy/BP_Goblin.BP_Goblin_C" null (`KismetMathLibrary.RandomPointInBoundingBox` (`SceneComponent.K2_GetComponentLocation` _box) (`BoxComponent.GetScaledBoxExtent` _box)) (struct) false null))
  (bind _asbp_ennemy (cast `/Game/Blueprints/Ennemy/BP_Ennemy` _returnvalue))
  (set `/Game/Blueprints/Ennemy/BP_Ennemy.XpGain` (`self.XpGainGoblin`) _asbp_ennemy)
  (set `/Game/Blueprints/Ennemy/BP_Ennemy.Hp` (`KismetMathLibrary.Conv_IntToDouble` (* (`self.WaveLevel`) 11)) _asbp_ennemy)
  (message `/Game/Blueprints/BPI_GameManager_Enemy.IncrementEnemyCount` (`GameplayStatics.GetGameMode`)))

(event `Spawn Wave`
  (`KismetSystemLibrary.PrintString` "JE SPAWN LA WAVE")
  (`self.UpdateXpGain`)
  (set `self.WaveLevel` (+ (`self.WaveLevel`) 1))
  (for _ (range (+ (`KismetMathLibrary.FTrunc` (* (* (`self.WaveLevel`) (`self.NumGoblinToSpawn`)) 0.7)) 1))
    (`self.SpawnEnemy`)))

(fn `UpdateXpGain`
  (if (and (== (mod (`self.WaveLevel`) 5) 0) (!= (`self.WaveLevel`) 0))
    (set `self.XpGainGoblin` (* (`self.XpGainGoblin`) 3))))

(fn `UserConstructionScript`)