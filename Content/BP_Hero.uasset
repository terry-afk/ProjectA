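; BP_Hero is the player character Blueprint, handling jump, camera look, movement and run input through Enhanced Input.
; BeginPlay adds the IM_ThirdPerson mapping context to the first player controller's subsystem.
; Look input drives controller yaw and pitch with per-axis inversion flags, and movement follows the control rotation, with pitch zeroed for forward motion.
; The run action flips a Running flag that switches max walk speed between two values.
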(event `self.ReceiveBeginPlay`
  (bind _returnvalue (pcsubsystem `EnhancedInputLocalPlayerSubsystem` (`GameplayStatics.GetPlayerController` 0)))
  (`/Engine/EditorBlueprintResources/StandardMacros.IsValid` _returnvalue
    (:`Is Valid`
      (`EnhancedInputSubsystemInterface.AddMappingContext` _returnvalue "/Game/IM_ThirdPerson.IM_ThirdPerson" 0 (struct)))))

(event `EnhancedInput|/Game/IA_Jump`
  (params (ActionValue :type Boolean) (ElapsedSeconds :type "Float (double-precision)") (TriggeredSeconds :type "Float (double-precision)") (InputAction :type "InputAction Object Reference" :default "/Game/IA_Jump.IA_Jump"))
  (:`Started`
    (`self.Jump`))
  (:`Completed`
    (`self.StopJumping`)))

(event `EnhancedInput|/Game/IA_LookArround`
  (params (ActionValue :type "Vector2D Structure") (ElapsedSeconds :type "Float (double-precision)") (TriggeredSeconds :type "Float (double-precision)") (InputAction :type "InputAction Object Reference" :default "/Game/IA_LookArround.IA_LookArround"))
  (:`Triggered`
    (`self.AddControllerYawInput` (* ActionValue_X (`KismetMathLibrary.SelectFloat` -1.0 1.0 (`self.InvertCameraX`))))
    (`self.AddControllerPitchInput` (* ActionValue_Y (`KismetMathLibrary.SelectFloat` -1.0 1.0 (`self.InvertCameraY`))))))

(event `EnhancedInput|/Game/IA_MoveArround`
  (params (ActionValue :type "Vector2D Structure") (ElapsedSeconds :type "Float (double-precision)") (TriggeredSeconds :type "Float (double-precision)") (InputAction :type "InputAction Object Reference" :default "/Game/IA_MoveArround.IA_MoveArround"))
  (bind (_returnvalue_roll _returnvalue_pitch _returnvalue_yaw) (`KismetMathLibrary.BreakRotator` (`self.GetControlRotation`)))
  (:`Triggered`
    (`self.AddMovementInput` (`KismetMathLibrary.GetRightVector` (`self.GetControlRotation`)) ActionValue_X)
    (`self.AddMovementInput` (`KismetMathLibrary.GetForwardVector` (`KismetMathLibrary.MakeRotator` _returnvalue_roll 0.0 _returnvalue_yaw)) ActionValue_Y)))

(event `EnhancedInput|/Game/AI_Run`
  (params (ActionValue :type Boolean) (ElapsedSeconds :type "Float (double-precision)") (TriggeredSeconds :type "Float (double-precision)") (InputAction :type "InputAction Object Reference" :default "/Game/AI_Run.AI_Run"))
  (bind _charactermovement (`self.CharacterMovement`))
  (:`Triggered`
    (bind _output_get (set `self.Running` (not (`self.Running`))))
    (if _output_get
      (set `CharacterMovementComponent.MaxWalkSpeed` 600.0 _charactermovement)
      (else
        (set `CharacterMovementComponent.MaxWalkSpeed` 350.0 _charactermovement)))))

(fn `UserConstructionScript`)